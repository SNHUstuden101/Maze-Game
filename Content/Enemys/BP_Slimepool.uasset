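; BP_Slimepool is a temporary slime hazard that slows the player while they stand in it.
; Overlapping its Cube component lowers BP_PlayerChar's max walk speed and prints the new value, and leaving restores a hardcoded normal speed.
; The actor destroys itself after a fixed delay from BeginPlay, with no explicit speed reset at that point.
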(event `self.ReceiveBeginPlay`
  (`KismetSystemLibrary.Delay` 11.0)
  (`self.K2_DestroyActor`))

(event `self.Cube.OnComponentBeginOverlap`
  (params (OverlappedComponent :type "PrimitiveComponent Object Reference") (OtherActor :type "Actor Object Reference") (OtherComp :type "PrimitiveComponent Object Reference") (OtherBodyIndex :type Integer) (bFromSweep :type Boolean) (SweepResult :type "HitResult Structure (by ref)"))
  (bind _asbp_player_char (cast `/Game/Player/BP_PlayerChar` OtherActor))
  (bind _output_get (set `CharacterMovementComponent.MaxWalkSpeed` 100.0 (`Character.CharacterMovement` _asbp_player_char)))
  (`KismetSystemLibrary.PrintString` (`KismetStringLibrary.Conv_DoubleToString` _output_get)))

(event `self.Cube.OnComponentEndOverlap`
  (params (OverlappedComponent :type "PrimitiveComponent Object Reference") (OtherActor :type "Actor Object Reference") (OtherComp :type "PrimitiveComponent Object Reference") (OtherBodyIndex :type Integer))
  (bind _asbp_player_char (cast `/Game/Player/BP_PlayerChar` OtherActor))
  (set `CharacterMovementComponent.MaxWalkSpeed` 600.0 (`Character.CharacterMovement` _asbp_player_char)))

(fn `UserConstructionScript`)