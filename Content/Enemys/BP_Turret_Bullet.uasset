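; BP_Turret_Bullet is an enemy turret projectile that damages the player on contact.
; Its Sphere overlap casts the other actor to BP_PlayerChar, applies fixed damage with itself as causer, then destroys itself.
; Overlaps with other actors are ignored, while a Hit event destroys the bullet after a tiny delay.
; A timed delay from BeginPlay limits the bullet's lifetime to a few seconds.
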(event `self.ReceiveBeginPlay`
  (`KismetSystemLibrary.Delay` 5.0)
  (`self.K2_DestroyActor`))

(event `self.Sphere.OnComponentBeginOverlap`
  (params (OverlappedComponent :type "PrimitiveComponent Object Reference") (OtherActor :type "Actor Object Reference") (OtherComp :type "PrimitiveComponent Object Reference") (OtherBodyIndex :type Integer) (bFromSweep :type Boolean) (SweepResult :type "HitResult Structure (by ref)"))
  (`|ExecutionSequence`
    (:`then_0`
      (bind _asbp_player (cast `/Game/Player/BP_PlayerChar` OtherActor))
      (`GameplayStatics.ApplyDamage` _asbp_player 10.0 null self)
      (`self.K2_DestroyActor`))))

(event `self.ReceiveHit`
  (params (MyComp :type "PrimitiveComponent Object Reference") (Other :type "Actor Object Reference") (OtherComp :type "PrimitiveComponent Object Reference") (bSelfMoved :type Boolean) (HitLocation :type "Vector Structure") (HitNormal :type "Vector Structure") (NormalImpulse :type "Vector Structure") (Hit :type "HitResult Structure (by ref)"))
  (`KismetSystemLibrary.Delay` 0.01)
  (`self.K2_DestroyActor`))

(fn `UserConstructionScript`)