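; Swinging axe hazard that swings through 180 degrees and deals damage to actors that overlap its box.
; A timeline started on BeginPlay lerps the Arrow's pitch, with a delay off its update triggering reversal and its finish calling play again.
; A DoOnce shared by all overlapping actors gates the damage and resets shortly after an overlap ends.
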(event `self.Box.OnComponentBeginOverlap`
  (params (OverlappedComponent :type "PrimitiveComponent Object Reference") (OtherActor :type "Actor Object Reference") (OtherComp :type "PrimitiveComponent Object Reference") (OtherBodyIndex :type Integer) (bFromSweep :type Boolean) (SweepResult :type "HitResult Structure (by ref)"))
  (`/Engine/EditorBlueprintResources/StandardMacros.DoOnce` false :!label _label
    (:`Completed`
      (`GameplayStatics.ApplyDamage` OtherActor 25.0 null self))))

(event `self.Box.OnComponentEndOverlap`
  (params (OverlappedComponent :type "PrimitiveComponent Object Reference") (OtherActor :type "Actor Object Reference") (OtherComp :type "PrimitiveComponent Object Reference") (OtherBodyIndex :type Integer))
  (`KismetSystemLibrary.Delay` 0.4)
  (goto _label :!via `Reset`))

(event `self.ReceiveBeginPlay`
  (`self.Axe_Play`))

(event `Axe_Play`
  (bind (_direction _alpha) (`Timeline|Timeline` :!label _label_2)
    (:`Update`
      (`SceneComponent.K2_SetRelativeRotation` (`self.Arrow`) (`KismetMathLibrary.MakeRotator` 0.0 (`KismetMathLibrary.Lerp` 0.0 -180.0 _alpha)) false false)
      (`KismetSystemLibrary.Delay` 2.0)
      (`self.Axe_Reverse`))
    (:`Finished`
      (`self.Axe_Play`))))

(event `Axe_Reverse`
  (goto _label_2 :!via `Reverse`))

(fn `UserConstructionScript`)