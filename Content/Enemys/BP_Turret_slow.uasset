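; BP_Turret_slow is an enemy turret that tracks the player and periodically fires slimeballs while the player is inside its detection box.
; Box overlap begin starts two looping timers by function name, and overlap end clears both.
; The fast timer rotates the Pivot from the actor's location toward player 0, and the slower one spawns BP_Turret_Slimeball at the ProjectileSpawn transform.
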(event `Fire`
  (`|SpawnActorFromClass` "/Game/Enemys/BP_Turret_Slimeball.BP_Turret_Slimeball_C" (`SceneComponent.K2_GetComponentToWorld` (`self.projectile spawn`)) "Undefined" "MultiplyWithRoot" null null))

(event `Followplayer`
  (`SceneComponent.K2_SetWorldRotation` (`self.pivot`) (`KismetMathLibrary.FindLookAtRotation` (`self.K2_GetActorLocation`) (`self.K2_GetActorLocation` (`GameplayStatics.GetPlayerCharacter` 0))) false false))

(event `self.Box.OnComponentBeginOverlap`
  (params (OverlappedComponent :type "PrimitiveComponent Object Reference") (OtherActor :type "Actor Object Reference") (OtherComp :type "PrimitiveComponent Object Reference") (OtherBodyIndex :type Integer) (bFromSweep :type Boolean) (SweepResult :type "HitResult Structure (by ref)"))
  (cast `/Game/Player/BP_PlayerChar` OtherActor)
  (`KismetSystemLibrary.K2_SetTimer` null "Followplayer" 0.05 true)
  (`KismetSystemLibrary.K2_SetTimer` null "Fire" 5.0 true))

(event `self.Box.OnComponentEndOverlap`
  (params (OverlappedComponent :type "PrimitiveComponent Object Reference") (OtherActor :type "Actor Object Reference") (OtherComp :type "PrimitiveComponent Object Reference") (OtherBodyIndex :type Integer))
  (cast `/Game/Player/BP_PlayerChar` OtherActor)
  (`KismetSystemLibrary.K2_ClearTimer` null "Followplayer")
  (`KismetSystemLibrary.K2_ClearTimer` null "Fire"))

(fn `UserConstructionScript`)