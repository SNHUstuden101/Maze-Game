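; BP_pickup_Colors is a colored, physics-driven cube that can be picked up and dropped through interact interface events.
; Interacting, if the passed reference is not already holding, sets its IsHolding flag, disables the cube's physics and collision, and snaps it to that reference's Arrow1.
; Dropping detaches the actor and restores collision and physics, without clearing IsHolding.
; The construction script applies PickupColor through a dynamic material instance.
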(event `/Game/Interfaces/Interface_INT.INT_interact`
  (params (REF :type "/Game/Player/BP_PlayerChar Object Reference"))
  (bind _cube (`self.Cube`))
  (if (not (`/Game/Player/BP_PlayerChar.Is Holding` REF))
    (set `/Game/Player/BP_PlayerChar.Is Holding` true REF)
    (`PrimitiveComponent.SetSimulatePhysics` _cube false)
    (`PrimitiveComponent.SetCollisionEnabled` _cube "NoCollision")
    (`SceneComponent.K2_AttachToComponent` _cube (`/Game/Player/BP_PlayerChar.Arrow1` REF) "None" "SnapToTarget" "KeepRelative" "KeepRelative" true)))

(event `/Game/Interfaces/Interface_INT.INT_Drop`
  (params (`Player ref` :type "/Game/Player/BP_PlayerChar Object Reference"))
  (bind _cube (`self.Cube`))
  (`self.K2_DetachFromActor` "KeepWorld" "KeepWorld" "KeepWorld")
  (`PrimitiveComponent.SetCollisionEnabled` _cube "QueryAndPhysics")
  (`PrimitiveComponent.SetSimulatePhysics` _cube true))

(fn `UserConstructionScript`
  (bind _returnvalue (`PrimitiveComponent.CreateDynamicMaterialInstance` (`self.Cube`) 0 "/Game/Material/Mat_color.Mat_color" "None"))
  (bind _output_get (set `self.Color DMI` _returnvalue))
  (`MaterialInstanceDynamic.SetVectorParameterValue` _output_get "Color" (`self.Pickup Color`)))