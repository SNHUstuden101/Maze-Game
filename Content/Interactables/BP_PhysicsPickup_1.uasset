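; Physics pickup interactable whose cube can be carried by the interacting actor and dropped back into the world.
; On interact, if the interactor is not already holding, the cube disables physics and collision, snaps to its Arrow1 component keeping relative rotation, and sets IsHolding.
; On drop, the actor detaches keeping world transform and restores the cube's collision and physics, leaving IsHolding untouched.
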(event `/Game/Interfaces/Interface_INT.INT_interact`
  (params (REF :type "/Game/Player/BP_PlayerChar Object Reference"))
  (bind _cube (`self.Cube`))
  (if (not (`/Game/Player/BP_PlayerChar.Is Holding` REF))
    (`PrimitiveComponent.SetSimulatePhysics` _cube false)
    (`PrimitiveComponent.SetCollisionEnabled` _cube "NoCollision")
    (`SceneComponent.K2_AttachToComponent` (`self.Cube`) (`/Game/Player/BP_PlayerChar.Arrow1` REF) "None" "SnapToTarget" "KeepRelative" "KeepRelative" true)
    (set `/Game/Player/BP_PlayerChar.Is Holding` true REF)))

(event `/Game/Interfaces/Interface_INT.INT_Drop`
  (params (`Player ref` :type "/Game/Player/BP_PlayerChar Object Reference"))
  (bind _cube (`self.Cube`))
  (`self.K2_DetachFromActor` "KeepWorld" "KeepWorld" "KeepWorld")
  (`PrimitiveComponent.SetCollisionEnabled` _cube "QueryAndPhysics")
  (`PrimitiveComponent.SetSimulatePhysics` _cube true))

(fn `UserConstructionScript`)