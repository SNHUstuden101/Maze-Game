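; Pressure plate interactable that unlocks a linked target door while the player character stands on it and locks it again when they step off.
; Overlap begin and end events set the door's unlock flag and play or reverse a timeline that sinks and raises the button mesh.
; The construction script tints the button through a dynamic material instance, and a debug message prints if no door is linked.
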(event `self.Overlap.OnComponentBeginOverlap`
  (params (OverlappedComponent :type "PrimitiveComponent Object Reference") (OtherActor :type "Actor Object Reference") (OtherComp :type "PrimitiveComponent Object Reference") (OtherBodyIndex :type Integer) (bFromSweep :type Boolean) (SweepResult :type "HitResult Structure (by ref)"))
  (bind _targetdoor (`self.TargetDoor`))
  (cast `/Game/Player/BP_PlayerChar` OtherActor)
  (`/Engine/EditorBlueprintResources/StandardMacros.IsValid` _targetdoor
    (:`Is Valid`
      (set `/Game/Interactables/AnimatedInteractables/BP_Button_Door.IsUnlocked` true _targetdoor)
      (bind (_direction _buttontrack) (`Timeline|ButtonPress` :!label _label)
        (:`Update`
          (`SceneComponent.K2_SetRelativeLocation` (`self.Button`) (`KismetMathLibrary.MakeVector` 0.0 0.0 (`KismetMathLibrary.Lerp` 3.7 1.3 _buttontrack)) false false))))
    (:`Is Not Valid`
      (`KismetSystemLibrary.PrintString` "Forgot to link door"))))

(event `self.Overlap.OnComponentEndOverlap`
  (params (OverlappedComponent :type "PrimitiveComponent Object Reference") (OtherActor :type "Actor Object Reference") (OtherComp :type "PrimitiveComponent Object Reference") (OtherBodyIndex :type Integer))
  (bind _targetdoor (`self.TargetDoor`))
  (cast `/Game/Player/BP_PlayerChar` OtherActor)
  (`/Engine/EditorBlueprintResources/StandardMacros.IsValid` _targetdoor
    (:`Is Valid`
      (set `/Game/Interactables/AnimatedInteractables/BP_Button_Door.IsUnlocked` false _targetdoor)
      (goto _label :!via `Reverse`))))

(fn `UserConstructionScript`
  (bind _returnvalue (`PrimitiveComponent.CreateDynamicMaterialInstance` (`self.Button`) 0 "/Game/Material/Mat_color.Mat_color" "None"))
  (bind _output_get (set `self.Color DMI` _returnvalue))
  (`MaterialInstanceDynamic.SetVectorParameterValue` _output_get "Color" (`self.Pickup Color`)))