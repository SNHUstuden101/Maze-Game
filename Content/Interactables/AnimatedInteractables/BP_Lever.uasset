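; Interactable lever that unlocks and relocks a linked TargetDoor.
; Each interact call alternates through a FlipFlop, setting the door's IsUnlocked and the lever's own unlocked flag while a Timeline plays or reverses to pitch the Arrow component.
; A missing door link prints a warning only on the unlock branch.
; The construction script tints the lever with PickupColor through a dynamic material instance; UpdateDoorAngle is a stub returning zero.
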(event `/Game/Interfaces/Interface_INT.INT_interact`
  (params (REF :type "/Game/Player/BP_PlayerChar Object Reference"))
  (bind _targetdoor (`self.TargetDoor`))
  (set `self.LEVER UNLOCKED` true)
  (`/Engine/EditorBlueprintResources/StandardMacros.FlipFlop`
    (:`A`
      (`/Engine/EditorBlueprintResources/StandardMacros.IsValid` _targetdoor
        (:`Is Valid`
          (set `/Game/Interactables/AnimatedInteractables/BP_Button_Door.IsUnlocked` true _targetdoor)
          (bind (_direction _alpha) (`Timeline|Timeline` :!label _label)
            (:`Update`
              (`SceneComponent.K2_SetRelativeRotation` (`self.Arrow`) (`KismetMathLibrary.MakeRotator` 0.0 (`KismetMathLibrary.Lerp` 90.0 50.0 _alpha)) false false))))
        (:`Is Not Valid`
          (`KismetSystemLibrary.PrintString` "Forgot to link door"))))
    (:`B`
      (`/Engine/EditorBlueprintResources/StandardMacros.IsValid` _targetdoor
        (:`Is Valid`
          (set `/Game/Interactables/AnimatedInteractables/BP_Button_Door.IsUnlocked` false _targetdoor)
          (set `self.LEVER UNLOCKED` false)
          (goto _label :!via `Reverse`))))))

(fn `Update door angle`
  (params (self2 :type "Actor Object Reference"))
  (returns (ReturnValue :type "Float (double-precision)"))
  (return 0.0))

(fn `UserConstructionScript`
  (bind _returnvalue (`PrimitiveComponent.CreateDynamicMaterialInstance` (`self.Lever`) 0 "/Game/Material/Mat_color.Mat_color" "None"))
  (bind _output_get (set `self.Color DMI` _returnvalue))
  (`MaterialInstanceDynamic.SetVectorParameterValue` _output_get "Color" (`self.Pickup Color`)))